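; Tunable FM radio prop with eight stations: F toggles a camera zoom onto the radio that freezes player walking, plus an emissive light marked unimplemented.
; Arrow keys or mouse wheel step Frequency within limits, moving the needle and dial.
; Once F opens a gate, Tick maps Frequency through nested branches to station volumes, blending in randomized white noise near each station and modulating its pitch and volume.
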(event `Key|F`
  ;[0.385 0.385 0.385] -               FM RADIO     - Needle and Dial -     EIGHT RADIO STATIONS     -
  ;;[1 0.9283 0.007025] Light - NOT IMPLIMENTED
  (:`Pressed`
    (`/Engine/EditorBlueprintResources/StandardMacros.FlipFlop`
      (:`A`
        (`MaterialInstanceDynamic.SetVectorParameterValue` (`self.ToggleEmissiveOn`) "RadioLight" (struct :`R` 0.99 :`G` 0.99 :`B` 0.99 :`A` 1.0)))
      (:`B`
        (`MaterialInstanceDynamic.SetVectorParameterValue` (`self.ToggleEmissiveOn`) "RadioLight" (struct :`A` 1.0))))))

(event `self.ReceiveTick`
  (params (DeltaSeconds :type "Float (single-precision)"))
  (bind _returnvalue (`KismetMathLibrary.RandomFloatInRange` -0.5 0.1))
  (bind _station_01 (`self.Station_01`))
  (bind _frequency (`self.Frequency`))
  (bind _turnonclick (`self.TurnOnClick`))
  (bind _wnoise (`self.WNoise`))
  (bind _station_01_2 (`self.Station_01`))
  (bind _station_01_3 (`self.Station_01`))
  (bind _station_01_4 (`self.Station_01`))
  (bind _station_02 (`self.Station_02`))
  (bind _station_02_2 (`self.Station_02`))
  (bind _station_02_3 (`self.Station_02`))
  (bind _station_03 (`self.Station_03`))
  (bind _station_03_2 (`self.Station_03`))
  (bind _station_03_3 (`self.Station_03`))
  (bind _station_04 (`self.Station_04`))
  (bind _station_04_2 (`self.Station_04`))
  (bind _station_04_3 (`self.Station_04`))
  (bind _station_05 (`self.Station_05`))
  (bind _station_05_2 (`self.Station_05`))
  (bind _station_05_3 (`self.Station_05`))
  (bind _station_06 (`self.Station_06`))
  (bind _station_06_2 (`self.Station_06`))
  (bind _station_06_3 (`self.Station_06`))
  (bind _station_07 (`self.Station_07`))
  (bind _station_07_2 (`self.Station_07`))
  (bind _station_07_3 (`self.Station_07`))
  (bind _station_08 (`self.Station_08`))
  (bind _station_08_2 (`self.Station_08`))
  (bind _station_08_3 (`self.Station_08`))
  ;[0.385 0.385 0.385] -               FM RADIO     - Needle and Dial -     EIGHT RADIO STATIONS     -
  ;;[0.02489 1 0] OnGate
  (`/Engine/EditorBlueprintResources/StandardMacros.Gate` true :!label _label
    (:`Exit`
      ;;[0.8546 1 0.1046] Activate Audio
      (`ActorComponent.Activate` _station_01 false)
      (`ActorComponent.Activate` (`self.Station_02`) false)
      (`ActorComponent.Activate` (`self.Station_03`) false)
      (`ActorComponent.Activate` (`self.Station_04`) false)
      (`ActorComponent.Activate` (`self.Station_05`) false)
      (`ActorComponent.Activate` (`self.Station_06`) false)
      (`ActorComponent.Activate` (`self.Station_08`) false)
      (`ActorComponent.Activate` (`self.WNoise`) false)
      (`ActorComponent.Activate` (`self.Station_07`) false)
      (`AudioComponent.AdjustVolume` _station_01 0.0 0.0)
      (`AudioComponent.AdjustVolume` (`self.Station_02`) 0.0 0.0)
      (`AudioComponent.AdjustVolume` (`self.Station_03`) 0.0 0.0)
      (`AudioComponent.AdjustVolume` (`self.Station_04`) 0.0 0.0)
      (`AudioComponent.AdjustVolume` (`self.Station_05`) 0.0 0.0)
      (`AudioComponent.AdjustVolume` (`self.Station_06`) 0.0 0.0)
      (`AudioComponent.AdjustVolume` (`self.Station_08`) 0.0 0.0)
      (`AudioComponent.AdjustVolume` (`self.WNoise`) 0.0 0.0)
      (`AudioComponent.AdjustVolume` (`self.Station_07`) 0.0 0.0)
      (`|ExecutionSequence`
        (:`then_0`
          ;;[0.8546 1 0.1046] Can Tune
          (if (== _frequency 1)
            (set `self.CanTuneUp` true)
            (set `self.CanTuneDown` false)))
        (:`then_1`
          (if (> _frequency 1)
            (set `self.CanTuneUp` true)
            (set `self.CanTuneDown` true)))
        (:`then_2`
          (if (> _frequency 41)
            (set `self.CanTuneDown` true)
            (set `self.CanTuneUp` false)))
        (:`then_3`
          ;;[1 1 1] Branch
          (if (!= (`self.Frequency`) 1)
            ;;[1 1 1] ON Click
            (`|ExecutionSequence`
              (:`then_0`
                (`/Engine/EditorBlueprintResources/StandardMacros.DoOnce` false
                  (:`Completed`
                    (`AudioComponent.AdjustVolume` _turnonclick 0.0 15.0)
                    (`ActorComponent.Activate` _turnonclick false))))
              (:`then_1`
                (if (!= (`self.Frequency`) 2)
                  ;;[1 1 1] White Noise
                  (`|ExecutionSequence`
                    (:`then_0`
                      (`AudioComponent.AdjustVolume` (`self.WNoise`) 0.0 0.5))
                    (:`then_1`
                      ;;[1 0.0374 0.7188] Track 1
                      (if (!= (`self.Frequency`) 5)
                        (`AudioComponent.AdjustVolume` _station_01_3 0.0 0.0)
                        (if (!= (`self.Frequency`) 6)
                          (`AudioComponent.AdjustVolume` _station_01_2 0.0 0.0)
                          (if (!= (`self.Frequency`) 7)
                            (`AudioComponent.AdjustVolume` _station_01_4 0.0 0.0)
                            ;;[0.02856 1 0.6683] Track 2
                            (if (!= (`self.Frequency`) 8)
                              (`AudioComponent.AdjustVolume` _station_02_2 0.0 0.0)
                              (if (!= (`self.Frequency`) 9)
                                (`AudioComponent.AdjustVolume` _station_02_3 0.0 0.0)
                                (if (!= (`self.Frequency`) 10)
                                  (`AudioComponent.AdjustVolume` _station_02 0.0 0.0)
                                  ;;[0.02856 1 0.6683] Track 3
                                  (if (!= (`self.Frequency`) 16)
                                    (`AudioComponent.AdjustVolume` _station_03_2 0.0 0.0)
                                    (if (!= (`self.Frequency`) 17)
                                      (`AudioComponent.AdjustVolume` _station_03_3 0.0 0.0)
                                      (if (!= (`self.Frequency`) 18)
                                        (`AudioComponent.AdjustVolume` _station_03 0.0 0.0)
                                        ;;[1 0.0374 0.7188] Track 4
                                        (if (!= (`self.Frequency`) 21)
                                          (`AudioComponent.AdjustVolume` _station_04_2 0.0 0.0)
                                          (if (!= (`self.Frequency`) 22)
                                            (`AudioComponent.AdjustVolume` _station_04_3 0.0 0.0)
                                            (if (!= (`self.Frequency`) 23)
                                              (`AudioComponent.AdjustVolume` _station_04 0.0 0.0)
                                              ;;[1 0.0374 0.7188] Track 5
                                              (if (!= (`self.Frequency`) 25)
                                                (`AudioComponent.AdjustVolume` _station_05_3 0.0 0.0)
                                                (if (!= (`self.Frequency`) 26)
                                                  (`AudioComponent.AdjustVolume` _station_05 0.0 0.0)
                                                  (if (!= (`self.Frequency`) 27)
                                                    (`AudioComponent.AdjustVolume` _station_05_2 0.0 0.0)
                                                    ;;[0.02856 1 0.6683] Track 6
                                                    (if (!= (`self.Frequency`) 28)
                                                      (`AudioComponent.AdjustVolume` _station_06_3 0.0 0.0)
                                                      (if (!= (`self.Frequency`) 29)
                                                        (`AudioComponent.AdjustVolume` _station_06 0.0 0.0)
                                                        (if (!= (`self.Frequency`) 30)
                                                          (`AudioComponent.AdjustVolume` _station_06_2 0.0 0.0)
                                                          ;;[0.02856 1 0.6683] Track 7
                                                          (if (!= (`self.Frequency`) 32)
                                                            (`AudioComponent.AdjustVolume` _station_07_3 0.0 0.0)
                                                            (if (!= (`self.Frequency`) 33)
                                                              (`AudioComponent.AdjustVolume` _station_07_2 0.0 0.0)
                                                              (if (!= (`self.Frequency`) 34)
                                                                (`AudioComponent.AdjustVolume` _station_07 0.0 0.0)
                                                                ;;[1 0.0374 0.7188] Track 8
                                                                (if (!= (`self.Frequency`) 37)
                                                                  (`AudioComponent.AdjustVolume` _station_08_2 0.0 0.0)
                                                                  (if (!= (`self.Frequency`) 38)
                                                                    (`AudioComponent.AdjustVolume` _station_08_3 0.0 0.0)
                                                                    (if (!= (`self.Frequency`) 39)
                                                                      (`AudioComponent.AdjustVolume` _station_08 0.0 0.0)
                                                                      (if (>= (`self.Frequency`) 41)
                                                                        (set `self.CanTuneUp` false))
                                                                      (else
                                                                        (`|ExecutionSequence`
                                                                          (:`then_0`
                                                                            (`AudioComponent.AdjustVolume` _station_08 0.0 0.5))
                                                                          (:`then_1`
                                                                            (`AudioComponent.AdjustVolume` (`self.WNoise`) 0.0 (`KismetMathLibrary.RandomFloatInRange` 0.0 0.25))))))
                                                                    (else
                                                                      (`|ExecutionSequence`
                                                                        (:`then_0`
                                                                          (`AudioComponent.AdjustVolume` _station_08_3 0.0 1.0))
                                                                        (:`then_1`
                                                                          (`AudioComponent.AdjustVolume` (`self.WNoise`) 0.0 0.0)))))
                                                                  (else
                                                                    (`|ExecutionSequence`
                                                                      (:`then_0`
                                                                        (`AudioComponent.AdjustVolume` _station_08_2 0.0 0.5))
                                                                      (:`then_1`
                                                                        (`AudioComponent.AdjustVolume` (`self.WNoise`) 0.0 (`KismetMathLibrary.RandomFloatInRange` 0.0 0.25))))))
                                                                (else
                                                                  (`|ExecutionSequence`
                                                                    (:`then_0`
                                                                      (`AudioComponent.AdjustVolume` _station_07 0.0 0.5))
                                                                    (:`then_1`
                                                                      (`AudioComponent.AdjustVolume` (`self.WNoise`) 0.0 (`KismetMathLibrary.RandomFloatInRange` 0.0 0.25))))))
                                                              (else
                                                                (`|ExecutionSequence`
                                                                  (:`then_0`
                                                                    (`AudioComponent.AdjustVolume` _station_07_2 0.0 1.0))
                                                                  (:`then_1`
                                                                    (`AudioComponent.AdjustVolume` (`self.WNoise`) 0.0 0.0)))))
                                                            (else
                                                              (`|ExecutionSequence`
                                                                (:`then_0`
                                                                  (`AudioComponent.AdjustVolume` _station_07_3 0.0 0.5))
                                                                (:`then_1`
                                                                  (`AudioComponent.AdjustVolume` (`self.WNoise`) 0.0 (`KismetMathLibrary.RandomFloatInRange` 0.0 0.25))))))
                                                          (else
                                                            (`|ExecutionSequence`
                                                              (:`then_0`
                                                                (`AudioComponent.AdjustVolume` _station_06_2 0.0 0.5))
                                                              (:`then_1`
                                                                (`AudioComponent.AdjustVolume` (`self.WNoise`) 0.0 (`KismetMathLibrary.RandomFloatInRange` 0.0 0.25))))))
                                                        (else
                                                          (`|ExecutionSequence`
                                                            (:`then_0`
                                                              (`AudioComponent.AdjustVolume` _station_06 0.0 1.0))
                                                            (:`then_1`
                                                              (`AudioComponent.AdjustVolume` (`self.WNoise`) 0.0 0.0)))))
                                                      (else
                                                        (`|ExecutionSequence`
                                                          (:`then_0`
                                                            (`AudioComponent.AdjustVolume` _station_06_3 0.0 0.0))
                                                          (:`then_1`
                                                            (`AudioComponent.AdjustVolume` (`self.WNoise`) 0.0 (`KismetMathLibrary.RandomFloatInRange` 0.0 0.25))))))
                                                    (else
                                                      (`|ExecutionSequence`
                                                        (:`then_0`
                                                          (`AudioComponent.AdjustVolume` _station_05_2 0.0 0.5))
                                                        (:`then_1`
                                                          (`AudioComponent.AdjustVolume` (`self.WNoise`) 0.0 (`KismetMathLibrary.RandomFloatInRange` 0.0 0.25))))))
                                                  (else
                                                    (`|ExecutionSequence`
                                                      (:`then_0`
                                                        (`AudioComponent.AdjustVolume` _station_05 0.0 1.0))
                                                      (:`then_1`
                                                        (`AudioComponent.AdjustVolume` (`self.WNoise`) 0.0 0.0)))))
                                                (else
                                                  (`|ExecutionSequence`
                                                    (:`then_0`
                                                      (`AudioComponent.AdjustVolume` _station_05_3 0.0 0.5))
                                                    (:`then_1`
                                                      (`AudioComponent.AdjustVolume` (`self.WNoise`) 0.0 (`KismetMathLibrary.RandomFloatInRange` 0.0 0.25))))))
                                              (else
                                                (`|ExecutionSequence`
                                                  (:`then_0`
                                                    (`AudioComponent.AdjustVolume` _station_04 0.0 0.5))
                                                  (:`then_1`
                                                    (`AudioComponent.AdjustVolume` (`self.WNoise`) 0.0 (`KismetMathLibrary.RandomFloatInRange` 0.0 0.25))))))
                                            (else
                                              (`|ExecutionSequence`
                                                (:`then_0`
                                                  (`AudioComponent.AdjustVolume` _station_04_3 0.0 1.0))
                                                (:`then_1`
                                                  (`AudioComponent.AdjustVolume` (`self.WNoise`) 0.0 0.0)))))
                                          (else
                                            (`|ExecutionSequence`
                                              (:`then_0`
                                                (`AudioComponent.AdjustVolume` _station_04_2 0.0 0.5))
                                              (:`then_1`
                                                (`AudioComponent.AdjustVolume` (`self.WNoise`) 0.0 (`KismetMathLibrary.RandomFloatInRange` 0.0 0.25))))))
                                        (else
                                          (`|ExecutionSequence`
                                            (:`then_0`
                                              (`AudioComponent.AdjustVolume` _station_03 0.0 0.5))
                                            (:`then_1`
                                              (`AudioComponent.AdjustVolume` (`self.WNoise`) 0.0 (`KismetMathLibrary.RandomFloatInRange` 0.0 0.25))))))
                                      (else
                                        (`|ExecutionSequence`
                                          (:`then_0`
                                            (`AudioComponent.AdjustVolume` _station_03_3 0.0 1.0))
                                          (:`then_1`
                                            (`AudioComponent.AdjustVolume` (`self.WNoise`) 0.0 0.0)))))
                                    (else
                                      (`|ExecutionSequence`
                                        (:`then_0`
                                          (`AudioComponent.AdjustVolume` _station_03_2 0.0 0.5))
                                        (:`then_1`
                                          (`AudioComponent.AdjustVolume` (`self.WNoise`) 0.0 (`KismetMathLibrary.RandomFloatInRange` 0.0 0.25))))))
                                  (else
                                    (`|ExecutionSequence`
                                      (:`then_0`
                                        (`AudioComponent.AdjustVolume` _station_02 0.0 0.5))
                                      (:`then_1`
                                        (`AudioComponent.AdjustVolume` (`self.WNoise`) 0.0 (`KismetMathLibrary.RandomFloatInRange` 0.0 0.25))))))
                                (else
                                  (`|ExecutionSequence`
                                    (:`then_0`
                                      (`AudioComponent.AdjustVolume` _station_02_3 0.0 1.0))
                                    (:`then_1`
                                      (`AudioComponent.AdjustVolume` (`self.WNoise`) 0.0 0.0)))))
                              (else
                                (`|ExecutionSequence`
                                  (:`then_0`
                                    (`AudioComponent.AdjustVolume` _station_02_2 0.0 0.5))
                                  (:`then_1`
                                    (`AudioComponent.AdjustVolume` (`self.WNoise`) 0.0 (`KismetMathLibrary.RandomFloatInRange` 0.0 0.25))))))
                            (else
                              (`|ExecutionSequence`
                                (:`then_0`
                                  (`AudioComponent.AdjustVolume` _station_01_4 0.0 0.5))
                                (:`then_1`
                                  (`AudioComponent.AdjustVolume` (`self.WNoise`) 0.0 (`KismetMathLibrary.RandomFloatInRange` 0.0 0.25))))))
                          (else
                            (`|ExecutionSequence`
                              (:`then_0`
                                (`AudioComponent.AdjustVolume` _station_01_2 0.0 1.0))
                              (:`then_1`
                                (`AudioComponent.AdjustVolume` (`self.WNoise`) 0.0 0.0)))))
                        (else
                          (`|ExecutionSequence`
                            (:`then_0`
                              (`AudioComponent.AdjustVolume` _station_01_3 0.0 0.5))
                            (:`then_1`
                              (`AudioComponent.AdjustVolume` (`self.WNoise`) 0.0 (`KismetMathLibrary.RandomFloatInRange` 0.0 0.25)))))))))))))
        (:`then_4`
          ;;[0.8546 1 0.1046] Noise Modulator
          (`AudioComponent.SetPitchMultiplier` _wnoise _returnvalue)
          (set `AudioComponent.VolumeMultiplier` _returnvalue _wnoise))))))

(event `Key|F`
  (bind _returnvalue (`GameplayStatics.GetPlayerController` 0))
  ;[0.385 0.385 0.385] -               FM RADIO     - Needle and Dial -     EIGHT RADIO STATIONS     -
  ;;[0.8546 1 0.1046] Enable Input
  (:`Pressed`
    (`|ExecutionSequence`
      (:`then_0`
        (`self.EnableInput` _returnvalue)
        (`/Engine/EditorBlueprintResources/StandardMacros.FlipFlop`
          (:`A`
            ;;[0.8546 1 0.1046] ZoomIn Radio
            (`PlayerController.SetViewTargetWithBlend` (`GameplayStatics.GetPlayerController` 0) self 1.0 "VTBlend_Linear" 0.0 true)
            (set `CharacterMovementComponent.MaxWalkSpeed` 0.0 (`Character.CharacterMovement` (`GameplayStatics.GetPlayerCharacter` 0)))
            ;;[0.8546 1 0.1046] Turn Static On
            (`AudioComponent.AdjustVolume` (`self.WNoise`) 0.0 0.0))
          (:`B`
            (`self.DisableInput` _returnvalue)
            ;;[0.8546 1 0.1046] ZoomOut Radio
            (`PlayerController.SetViewTargetWithBlend` (`GameplayStatics.GetPlayerController` 0) (`GameplayStatics.GetPlayerCharacter` 0) 1.0 "VTBlend_Linear" 0.0 true)
            (set `CharacterMovementComponent.MaxWalkSpeed` 300.0 (`Character.CharacterMovement` (`GameplayStatics.GetPlayerCharacter` 0)))))
        ;;[0.8546 1 0.1046] Text Tooltip
        (`SceneComponent.ToggleVisibility` (`self.TextRender1`) false)
        (`SceneComponent.ToggleVisibility` (`self.TextRender2`) false))
      (:`then_1`
        (goto _label :!via `Open`)))))

(event `Key|Right`
  ;[0.385 0.385 0.385] -               FM RADIO     - Needle and Dial -     EIGHT RADIO STATIONS     -
  ;;[1 0.085 0.085] Input Right
  ;;;[0.8546 1 0.1046] Get Input
  (:`Pressed`
    (if (`self.CanTuneUp`) :!label _label_2
      ;;;[0.8546 1 0.1046] Move Needle
      (`SceneComponent.AddLocalOffset` (`self.Needle`) (1.0 0.0 0.0) false)
      ;;;[0.8546 1 0.1046] Rotate Dial
      (`SceneComponent.AddLocalRotation` (`self.TuneDial`) (struct :`Yaw` 3.0) false)
      ;;;[0.8546 1 0.1046] Frequency
      (set `self.Frequency` (+ 1 (`self.Frequency`)))
      (if (== (`self.Frequency`) 5)
        _))))

(event `Key|Left`
  ;[0.385 0.385 0.385] -               FM RADIO     - Needle and Dial -     EIGHT RADIO STATIONS     -
  ;;[0.08585 0.505 0.09633] Input Left
  ;;;[0.8546 1 0.1046] Get Input
  (:`Pressed`
    (if (`self.CanTuneDown`) :!label _label_3
      ;;;[0.8546 1 0.1046] Move Needle
      (`SceneComponent.AddLocalOffset` (`self.Needle`) (-1.0 0.0 0.0) false)
      ;;;[0.8546 1 0.1046] Rotate Dial
      (`SceneComponent.AddLocalRotation` (`self.TuneDial`) (struct :`Yaw` -3.0) false)
      ;;;[0.8546 1 0.1046] Frequency
      (set `self.Frequency` (+ -1 (`self.Frequency`))))))

(event `Key|MouseScrollDown`
  ;[0.385 0.385 0.385] -               FM RADIO     - Needle and Dial -     EIGHT RADIO STATIONS     -
  ;;[0.08585 0.505 0.09633] Input Left
  ;;;[0.8546 1 0.1046] Get Input
  (:`Released`
    (goto _label_3)))

(event `Key|MouseScrollUp`
  ;[0.385 0.385 0.385] -               FM RADIO     - Needle and Dial -     EIGHT RADIO STATIONS     -
  ;;[1 0.085 0.085] Input Right
  ;;;[0.8546 1 0.1046] Get Input
  (:`Pressed`
    (goto _label_2)))

(fn `UserConstructionScript`
  (bind _returnvalue (`PrimitiveComponent.CreateDynamicMaterialInstance` (`self.StaticMesh1`) 0 null))
  (set `self.ToggleEmissiveOn` _returnvalue))